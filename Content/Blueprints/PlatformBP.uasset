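; PlatformBP is an actor that the player tilts through two input axes.
; TiltHorizontally adds its axis value to the actor's roll, and TiltVertically adds its value to the pitch, leaving the other rotation components as they are.
; Each input event applies the change directly with SetActorRotation, with no clamping or delta-time scaling.
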(event `InputAxis|TiltHorizontally`
  (params (AxisValue :type "Float (single-precision)"))
  (`self.SetActorRotation` (`KismetMathLibrary.MakeRot` (.pitch (`self.K2_GetActorRotation`)) (.yaw (`self.K2_GetActorRotation`)) (+ AxisValue (.roll (`self.K2_GetActorRotation`))))))

(event `InputAxis|TiltVertically`
  (params (AxisValue :type "Float (single-precision)"))
  (`self.SetActorRotation` (`KismetMathLibrary.MakeRot` (+ AxisValue (.pitch (`self.K2_GetActorRotation`))) (.yaw (`self.K2_GetActorRotation`)) (.roll (`self.K2_GetActorRotation`)))))

(fn `UserConstructionScript`)